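; Third-person shooter player controller that creates a hidden player score widget on BeginPlay and adds it to the viewport.
; Pressing Tab loops over the GameState PlayerArray, casts to BP_PlayerState and prints each player's ID and score on screen.
; Unconnected logic sketches an unfinished scoreboard that would create score items, refill the widget and toggle its visibility, so the widget stays hidden.
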(event `self.ReceiveBeginPlay`
  (bind _returnvalue (`|CreateWidget` "/Game/BluePrint/UI/BP_PlayerScoreWidget.BP_PlayerScoreWidget_C" (`GameplayStatics.GetPlayerController` 0)))
  (bind _output_get (set `self.PlayerScoreWidget` _returnvalue))
  (`Widget.SetVisibility` _output_get "Hidden")
  (`UserWidget.AddToViewport` _output_get 0))

(event `Key|Tab`
  (params (Key :type "Key Structure"))
  (:`Pressed`
    (for _array_element (`GameStateBase.PlayerArray` (`GameplayStatics.GetGameState`))
      (bind _asbp_player_state (cast `/Game/BluePrint/Player/BP_PlayerState` _array_element))
      (`KismetSystemLibrary.PrintString` (`KismetTextLibrary.Conv_TextToString` (`|FormatText` "PlayerId {id} Score: {Score}" (`PlayerState.PlayerId` _asbp_player_state) (`/Game/BluePrint/Player/BP_PlayerState.PlayerScore` _asbp_player_state))) true false))))

(fn `UserConstructionScript`)