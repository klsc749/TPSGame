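; Target actor that awards points to the player who damages it and then destroys itself.
; On BeginPlay it binds a handler to its own OnTakeAnyDamage event.
; The handler casts the damage causer to BaseCharacter and its PlayerState to BP_PlayerState, adds a fixed amount to PlayerScore, and prints a message if either cast fails.
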(event `CustomEvent_0` :!signature `self.OnTakeAnyDamage`
  (params (DamagedActor :type "Actor Object Reference") (Damage :type "Float (double-precision)") (DamageType :type "DamageType Object Reference") (InstigatedBy :type "Controller Object Reference") (DamageCauser :type "Actor Object Reference"))
  (bind _asbase_character (cast `BaseCharacter` DamageCauser)
    (:`then`
      (bind _asbp_player_state (cast `/Game/BluePrint/Player/BP_PlayerState` (`Pawn.PlayerState` _asbase_character))
        (:`then`
          (set `/Game/BluePrint/Player/BP_PlayerState.PlayerScore` (+ (`/Game/BluePrint/Player/BP_PlayerState.PlayerScore` _asbp_player_state) 5) _asbp_player_state)
          (`self.K2_DestroyActor`))
        (:`CastFailed`
          (`KismetSystemLibrary.PrintString` "Can't Cast To PlayerState"))))
    (:`CastFailed`
      (`KismetSystemLibrary.PrintString` "Can't Cast To BaseCharacter"))))

(event `self.ReceiveBeginPlay`
  (add `self.OnTakeAnyDamage` (delegate `CustomEvent_0`)))

(fn `UserConstructionScript`)